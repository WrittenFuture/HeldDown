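; BP_ToggleableLights is an actor holding a group of eight spot lights that switch on and off together.
; Every Tick it copies the IsLightsOn boolean to each light's visibility, without propagating to children.
; The flag is only read here, as BeginPlay and the construction script are empty and no graph sets it.
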(event `self.ReceiveBeginPlay`)

(event `self.ReceiveTick`
  (params (DeltaSeconds :type "Float (single-precision)"))
  (bind _islightson (`self.IsLightsOn`))
  (`SceneComponent.SetVisibility` (`self.SpotLight7`) _islightson false)
  (`SceneComponent.SetVisibility` (`self.SpotLight2`) _islightson false)
  (`SceneComponent.SetVisibility` (`self.SpotLight4`) _islightson false)
  (`SceneComponent.SetVisibility` (`self.SpotLight3`) _islightson false)
  (`SceneComponent.SetVisibility` (`self.SpotLight`) _islightson false)
  (`SceneComponent.SetVisibility` (`self.SpotLight1`) _islightson false)
  (`SceneComponent.SetVisibility` (`self.SpotLight5`) _islightson false)
  (`SceneComponent.SetVisibility` (`self.SpotLight11`) _islightson false))

(fn `UserConstructionScript`)