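; Street lights Blueprint that shows or hides its point lights according to the IsLightsOn flag.
; Tick applies the flag to PointLight and PointLight1 through PointLight4 every frame through a chain of SetVisibility calls, several repeating on PointLight, without propagating to children.
; Nothing in these graphs changes IsLightsOn, and BeginPlay, overlap and the construction script are empty.
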(event `self.ReceiveBeginPlay`)

(event `self.ReceiveTick`
  (params (DeltaSeconds :type "Float (single-precision)"))
  (bind _pointlight (`self.PointLight`))
  (bind _islightson (`self.IsLightsOn`))
  (`SceneComponent.SetVisibility` _pointlight _islightson false)
  (`SceneComponent.SetVisibility` _pointlight _islightson false)
  (`SceneComponent.SetVisibility` (`self.PointLight1`) _islightson false)
  (`SceneComponent.SetVisibility` _pointlight _islightson false)
  (`SceneComponent.SetVisibility` (`self.PointLight2`) _islightson false)
  (`SceneComponent.SetVisibility` _pointlight _islightson false)
  (`SceneComponent.SetVisibility` (`self.PointLight3`) _islightson false)
  (`SceneComponent.SetVisibility` _pointlight _islightson false)
  (`SceneComponent.SetVisibility` (`self.PointLight4`) _islightson false)
  (`SceneComponent.SetVisibility` _pointlight _islightson false)
  (`SceneComponent.SetVisibility` _pointlight _islightson false)
  (`SceneComponent.SetVisibility` _pointlight _islightson false))

(fn `UserConstructionScript`)